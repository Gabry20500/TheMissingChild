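; Interactable drawer Blueprint that slides itself and the player by an offset when the player interacts.
; Box overlap shows an interact widget and, for BP_Player, binds the player's interact dispatcher; end overlap clears all widgets.
; Interaction disables input, moves the player capsule and drawer root together via MoveComponentTo, then restores input.
; The move branch is always true, the stored initial position is unused, and nothing returns the drawer.
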(event `self.ReceiveBeginPlay`
  (set `self.InitialPos` (`SceneComponent.K2_GetComponentLocation` (`self.Mesh`)))
  (bind _returnvalue (`GameplayStatics.GetActorOfClass` "/Game/Player/BP_Player.BP_Player_C"))
  (set `self.PG_Ref` _returnvalue))

(event `self.Box.OnComponentBeginOverlap`
  (params (OverlappedComponent :type "PrimitiveComponent Object Reference") (OtherActor :type "Actor Object Reference") (OtherComp :type "PrimitiveComponent Object Reference") (OtherBodyIndex :type Integer) (bFromSweep :type Boolean) (SweepResult :type "HitResult Structure (by ref)"))
  (bind _returnvalue (`|CreateWidget` "/Game/PickUp/Interact_WG.Interact_WG_C"))
  (`UserWidget.AddToViewport` _returnvalue 0)
  (if (== (`GameplayStatics.GetObjectClass` OtherActor) "/Game/Player/BP_Player.BP_Player_C")
    (add `/Game/Player/BP_Player.InteractDispatcher` (`self.PG_Ref`) (delegate `CustomEvent_0`))
    (`KismetSystemLibrary.PrintString` "binded")))

(event `CustomEvent_0`
  (bind _defaultsceneroot (`self.DefaultSceneRoot`))
  (bind _returnvalue (`self.GetComponentByClass` (`self.PG_Ref`) "/Script/Engine.CapsuleComponent"))
  (`KismetSystemLibrary.PrintString` "called")
  (`self.DisableInput` (`self.PG_Ref`) null)
  (if true
    (`|ExecutionSequence`
      (:`then_0`
        (`KismetSystemLibrary.MoveComponentTo` _returnvalue (+ (`SceneComponent.K2_GetComponentLocation` _returnvalue) (`self.VectorOffSet`)) (`SceneComponent.K2_GetComponentRotation` _returnvalue) false false 2.0))
      (:`then_1`
        (`KismetSystemLibrary.MoveComponentTo` _defaultsceneroot (+ (`SceneComponent.K2_GetComponentLocation` _defaultsceneroot) (`self.VectorOffSet`)) (`SceneComponent.K2_GetComponentRotation` _defaultsceneroot) false false 2.0)))
    (`self.EnableInput` (`self.PG_Ref`) null)
    (else
      (`self.EnableInput` (`self.PG_Ref`) null))))

(event `self.Box.OnComponentEndOverlap`
  (params (OverlappedComponent :type "PrimitiveComponent Object Reference") (OtherActor :type "Actor Object Reference") (OtherComp :type "PrimitiveComponent Object Reference") (OtherBodyIndex :type Integer))
  (bind _pg_ref (`self.PG_Ref`))
  (`WidgetLayoutLibrary.RemoveAllWidgets`)
  (if (== (`GameplayStatics.GetObjectClass` null) "/Game/Player/BP_Player.BP_Player_C")
    (remove `/Game/Player/BP_Player.InteractDispatcher` _pg_ref (delegate `CustomEvent_0`))
    (`self.EnableInput` _pg_ref null)))

(fn `UserConstructionScript`)