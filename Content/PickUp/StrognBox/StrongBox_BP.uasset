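; StrongBox pickup actor Blueprint that displays up to two batteries according to its BatteryNum counter.
; Tick switches on BatteryNum every frame, hiding both battery components at zero, showing Battery1 at one and Battery2 at two.
; BeginPlay raises the count to one and then two on timed delays, with no player interaction involved.
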(event `self.ReceiveBeginPlay`
  (`KismetSystemLibrary.Delay` 2.0)
  (set `self.BatteryNum` 1)
  (`KismetSystemLibrary.Delay` 2.0)
  (set `self.BatteryNum` 2))

(event `self.ReceiveTick`
  (params (DeltaSeconds :type "Float (single-precision)"))
  (switch `int` (`self.BatteryNum`)
    (:`0`
      (`SceneComponent.SetVisibility` (`self.Battery1`) false false)
      (`SceneComponent.SetVisibility` (`self.Battery2`) false false))
    (:`1`
      (`SceneComponent.SetVisibility` (`self.Battery1`) true false))
    (:`2`
      (`SceneComponent.SetVisibility` (`self.Battery2`) true false))))

(fn `UserConstructionScript`)