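; StrongBoxDoor_BP is the door of a strongbox pickup that rotates based on the box's battery count.
; On BeginPlay it finds the StrongBox_BP actor in the level and caches the cast reference.
; Tick passes through a DoOnce before testing for two batteries, so the check runs only on the first tick and, if true, rotates the mesh half a turn.
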(event `self.ReceiveBeginPlay`
  (bind _returnvalue (`GameplayStatics.GetActorOfClass` "/Game/PickUp/StrognBox/StrongBox_BP.StrongBox_BP_C"))
  (bind _asstrong_box_bp (cast `/Game/PickUp/StrognBox/StrongBox_BP` _returnvalue))
  (set `self.As Strong Box BP` _asstrong_box_bp))

(event `self.ReceiveTick`
  (params (DeltaSeconds :type "Float (single-precision)"))
  (`/Engine/EditorBlueprintResources/StandardMacros.DoOnce` false
    (:`Completed`
      (if (== (`/Game/PickUp/StrognBox/StrongBox_BP.BatteryNum` (`self.As Strong Box BP`)) 2)
        (`SceneComponent.K2_AddWorldRotation` (`self.StaticMesh`) (struct :`Yaw` 180.0) false false)))))

(fn `UserConstructionScript`)