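; BP_Movable is an actor the player can drag, flagged through a Box trigger volume.
; While Done is false, overlap adds an Interact_Wg prompt, then sets DragItem and TargetMovable on BP_Player, leaving the drag itself outside this Blueprint.
; End overlap removes all widgets, not just the prompt, and clears DragItem but leaves TargetMovable set.
; The prompt appears before the player cast, so any overlapping actor triggers it.
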(event `self.Box.OnComponentBeginOverlap`
  (params (OverlappedComponent :type "PrimitiveComponent Object Reference") (OtherActor :type "Actor Object Reference") (OtherComp :type "PrimitiveComponent Object Reference") (OtherBodyIndex :type Integer) (bFromSweep :type Boolean) (SweepResult :type "HitResult Structure (by ref)"))
  (if (not (`self.Done`))
    (bind _returnvalue (`|CreateWidget` "/Game/PickUp/Movable/Interact_Wg.Interact_Wg_C"))
    (`UserWidget.AddToViewport` _returnvalue 0)
    (bind _asbp_player (cast `/Game/Player/BP_Player` OtherActor))
    (set `/Game/Player/BP_Player.DragItem?` true _asbp_player)
    (set `/Game/Player/BP_Player.targetMovable` self _asbp_player)))

(event `self.Box.OnComponentEndOverlap`
  (params (OverlappedComponent :type "PrimitiveComponent Object Reference") (OtherActor :type "Actor Object Reference") (OtherComp :type "PrimitiveComponent Object Reference") (OtherBodyIndex :type Integer))
  (`WidgetLayoutLibrary.RemoveAllWidgets`)
  (bind _asbp_player (cast `/Game/Player/BP_Player` OtherActor))
  (set `/Game/Player/BP_Player.DragItem?` false _asbp_player))

(fn `UserConstructionScript`)